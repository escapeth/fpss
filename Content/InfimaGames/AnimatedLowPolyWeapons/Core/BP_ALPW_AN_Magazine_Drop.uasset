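; Animation notify, shown as "Drop Magazine", that drops or restores a weapon's magazine during animations.
; It gets the magazine mesh component from the animated mesh's owner through a message call.
; When Drop is set, it spawns a magazine actor at that transform, copies the static mesh and materials, then hides the original.
; Otherwise it makes the original magazine visible again.
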(fn GetNotifyName
  (return "Drop Magazine"))

(fn ReceivedNotify
  (params (MeshComp :type Skeletal%20Mesh%20Component%20Object%20Reference) (Animation :type Anim%20Sequence%20Base%20Object%20Reference) (EventReference :type Anim%20Notify%20Event%20Reference%20Structure%20%28by%20ref%29))
  (Utilities|FlowControl|Sequence
    (:then_0
      (LocalVariables|SetActor%20Weapon (Components|GetOwner MeshComp) :!pinned true) ; Cache Weapon.
      (bind _returnvalue (Class|BPIALPWWEP|GetMeshComponentMagazine(Message) (LocalVariables|GetActor%20Weapon))) ; Cache the magazine static mesh component, so we can copy it later.
      (bind _output_get (LocalVariables|SetMesh%20Component%20Magazine _returnvalue))
      (Utilities|IsValid _output_get
        (:Is%20Valid
          (if (Variables|InfimaGames|AnimatedLowPolyWeapons|MagazineDrop|GetDrop)
            (bind _returnvalue_2 (Game|SpawnActorfromClass "/Game/InfimaGames/AnimatedLowPolyWeapons/Core/BP_ALPW_Magazine.BP_ALPW_Magazine_C" (Transformation|GetWorldTransform (LocalVariables|GetMesh%20Component%20Magazine)) "Undefined" 0 0 :!pinned true)) ; Spawn New Magazine. This drops the magazine, basically.
            (LocalVariables|SetMesh%20Magazine _returnvalue_2)
            (Components|StaticMesh|SetStaticMesh (Variables|/Game/InfimaGames/AnimatedLowPolyWeapons/Core/BP_ALPW_Magazine.BP_ALPW_Magazine_C|GetMesh%20Magazine (LocalVariables|GetMesh%20Magazine)) (Variables|/Script/Engine.StaticMeshComponent|GetStaticMesh (LocalVariables|GetMesh%20Component%20Magazine)) :!pinned true) ; Copy Static Mesh. Matches the visual magazine.
            (Utilities|FlowControl|Sequence
              (:then_0
                (for _index (range 0 (Rendering|Material|GetNumMaterials (Variables|/Game/InfimaGames/AnimatedLowPolyWeapons/Core/BP_ALPW_Magazine.BP_ALPW_Magazine_C|GetMesh%20Magazine (LocalVariables|GetMesh%20Magazine))))
                  (Rendering|Material|SetMaterial (Variables|/Game/InfimaGames/AnimatedLowPolyWeapons/Core/BP_ALPW_Magazine.BP_ALPW_Magazine_C|GetMesh%20Magazine (LocalVariables|GetMesh%20Magazine)) _index (Rendering|Material|GetMaterial (LocalVariables|GetMesh%20Component%20Magazine) _index))))
              (:then_1
                (Rendering|SetVisibility (LocalVariables|GetMesh%20Component%20Magazine) false false)))
            (else
              (Rendering|SetVisibility (LocalVariables|GetMesh%20Component%20Magazine) true false))))))
    (:then_1
      (return true))))