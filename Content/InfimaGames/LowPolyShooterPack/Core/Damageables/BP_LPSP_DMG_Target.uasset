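; Shooting target that drops when hit by point damage and pops back up after a random delay.
; A Lowered flag ignores repeat hits while down, and collapsed graphs show a hit text widget, play the lower and reset animations with sounds, and handle the timing.
; It counts as an assist target only while raised.
; On Health death, it spawns an optional destroyed version at the mesh's target socket.
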(event OnDeath(Health)
  ;[1 0.8203 0] Death
  (if (Utilities|IsValidClass (Variables|InfimaGames|LowPolyShooterPack|DamageableTarget|GetDestroyed%20Version%20Class))
    (Game|SpawnActorfromClass (Variables|InfimaGames|LowPolyShooterPack|DamageableTarget|GetDestroyed%20Version%20Class) (Transformation|GetSocketTransform (Variables|Default|GetTarget%20Mesh) "SOCKET_Target" "RTS_World") "AlwaysSpawn" 0 0) ; Spawn Destroyed
  ))

(event Game|Damage|EventPointDamage
  (params (Damage :type Float%20%28single-precision%29) (DamageType :type Damage%20Type%20Object%20Reference) (HitLocation :type Vector :default "0, 0, 0") (HitNormal :type Vector :default "0, 0, 0") (HitComponent :type Primitive%20Component%20Object%20Reference) (BoneName :type Name :default "None") (ShotFromDirection :type Vector :default "0, 0, 0") (InstigatedBy :type Controller%20Object%20Reference) (DamageCauser :type Actor%20Object%20Reference) (HitInfo :type Hit%20Result%20Structure%20%28by%20ref%29))
  ;[0.2656 1 0] Point Damage
  (|CallParentFunction Damage DamageType HitLocation HitNormal HitComponent BoneName ShotFromDirection InstigatedBy DamageCauser HitInfo)
  (if (not (Variables|InfimaGames|LowPolyShooterPack|Data|GetLowered))
    (Variables|InfimaGames|LowPolyShooterPack|Data|SetLowered true)
    (|CGraphSpawnHitText)
    (|CGraphLowerTargett)
    (|CGraphResetTarget)))

(fn ConstructionScript
  (|CallParentFunction))

(fn IsAssistTarget
  (return (not (Variables|InfimaGames|LowPolyShooterPack|Data|GetLowered))))