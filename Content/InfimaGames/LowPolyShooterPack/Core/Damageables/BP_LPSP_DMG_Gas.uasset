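; Damageable gas prop that ignites and propels itself when shot, then is killed by a further hit.
; The first point damage toggles two thrusters and activates flame audio and particles; any later point damage triggers the kill event on its Health component.
; BeginPlay randomizes both thrust strengths within set ranges, scaled by mesh mass, and the construction script randomizes the flame particle size.
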(event EventBeginPlay
  (bind _thruster_strength (Variables|InfimaGames|LowPolyShooterPack|Gas|GetThruster%20Strength))
  (bind _thruster_strength__sideways_ (Variables|InfimaGames|LowPolyShooterPack|Gas|GetThruster%20Strength%20%28Sideways%29))
  ;[1 0 0.07031 1 12] Begin Play
  (|CallParentFunction)
  (Variables|/Script/Engine.PhysicsThrusterComponent|SetThrustStrength (Variables|Default|GetThruster) (* (Math|Random|RandomFloatinRange (.x _thruster_strength) (.y _thruster_strength)) (Physics|GetMass (Variables|Character|GetMesh))))
  (Variables|/Script/Engine.PhysicsThrusterComponent|SetThrustStrength (Variables|Default|GetThruster%20Sideways) (* (Math|Random|RandomFloatinRange (.x _thruster_strength__sideways_) (.y _thruster_strength__sideways_)) (Physics|GetMass (Variables|Character|GetMesh)))))

(event Game|Damage|EventPointDamage
  (params (Damage :type Float%20%28single-precision%29) (DamageType :type Damage%20Type%20Object%20Reference) (HitLocation :type Vector :default "0, 0, 0") (HitNormal :type Vector :default "0, 0, 0") (HitComponent :type Primitive%20Component%20Object%20Reference) (BoneName :type Name :default "None") (ShotFromDirection :type Vector :default "0, 0, 0") (InstigatedBy :type Controller%20Object%20Reference) (DamageCauser :type Actor%20Object%20Reference) (HitInfo :type Hit%20Result%20Structure%20%28by%20ref%29))
  ;[0 0.3203 1 1 12] Damage (Point)
  (|CallParentFunction Damage DamageType HitLocation HitNormal HitComponent BoneName ShotFromDirection InstigatedBy DamageCauser HitInfo)
  (if (Variables|Data|GetbHit)
    (Default|EventKill (Variables|Default|GetHealth))
    (else
      (Variables|Data|SetbHit true)
      (Components|Activation|ToggleActive (Variables|Default|GetThruster))
      (Components|Activation|ToggleActive (Variables|Default|GetThruster%20Sideways))
      (Components|Activation|Activate (Variables|Default|GetFlames%20Audio) true)
      (Components|Activation|Activate (Variables|Default|GetFlames%20Particles) true))))

(fn ConstructionScript
  (bind _flame_particles__size_ (Variables|InfimaGames|LowPolyShooterPack|Gas|GetFlame%20Particles%20%28Size%29))
  (|CallParentFunction)
  (Transformation|SetWorldScale3D (Variables|Default|GetFlames%20Particles) (Math|Conversions|ToVector(Float) (Math|Random|RandomFloatinRange (.x _flame_particles__size_) (.y _flame_particles__size_)))))