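; Anim notify that plays a camera shake for the player whose pawn owns the animated mesh.
; On notify, it casts the mesh owner to a Pawn and its controller to a PlayerController, then starts a client camera shake with the configured class and scale.
; Owners without a player controller get no shake.
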(fn ReceivedNotify
  (params (MeshComp :type Skeletal%20Mesh%20Component%20Object%20Reference) (Animation :type Anim%20Sequence%20Base%20Object%20Reference) (EventReference :type Anim%20Notify%20Event%20Reference%20Structure%20%28by%20ref%29))
  (bind _returnvalue (Components|GetOwner MeshComp))
  (Utilities|FlowControl|Sequence
    (:then_0
      (Utilities|IsValid _returnvalue
        (:Is%20Valid
          (bind _aspawn (Utilities|Casting|CastToPawn _returnvalue))
          (Utilities|IsValid (Pawn|GetController _aspawn)
            (:Is%20Valid
              (bind _asplayer_controller (Utilities|Casting|CastToPlayerController (Pawn|GetController _aspawn)))
              (Game|Feedback|ClientStartCameraShake _asplayer_controller (Variables|Default|GetClass%20Shake) (Variables|Default|GetScale) "CameraLocal" "0, 0, 0"))))))
    (:then_1
      (return true))))