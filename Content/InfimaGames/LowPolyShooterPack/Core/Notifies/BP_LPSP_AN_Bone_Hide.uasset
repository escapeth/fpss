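; Animation notify in the Low Poly Shooter Pack that hides or shows a named bone on the animated skeletal mesh.
; When fired, it checks its Hidden flag and either hides the bone, terminating its physics body, or unhides it, then reports success.
; It displays as "Hide Bone" in the animation timeline.
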(fn ReceivedNotify
  (params (MeshComp :type Skeletal%20Mesh%20Component%20Object%20Reference) (Animation :type Anim%20Sequence%20Base%20Object%20Reference) (EventReference :type Anim%20Notify%20Event%20Reference%20Structure%20%28by%20ref%29))
  (Utilities|FlowControl|Sequence
    (:then_0
      (if (Variables|Default|GetHidden)
        (Components|SkinnedMesh|HideBonebyName MeshComp (Variables|Default|GetBone%20Name) "PBO_Term")
        (else
          (Components|SkinnedMesh|UnHideBonebyName MeshComp (Variables|Default|GetBone%20Name)))))
    (:then_1
      (return true))))

(fn GetNotifyName
  (return "Hide Bone"))