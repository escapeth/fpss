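; Animation notify for the Low Poly Shooter Pack that plays a footstep sound when triggered during an animation.
; After checking that the mesh, its anim instance and the sound are valid, it spawns the sound attached to the mesh at a named attach point.
; Sound, attach point, volume and pitch come from notify variables, and the notify always returns true, even when nothing plays.
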(fn ReceivedNotify
  (params (MeshComp :type Skeletal%20Mesh%20Component%20Object%20Reference) (Animation :type Anim%20Sequence%20Base%20Object%20Reference) (EventReference :type Anim%20Notify%20Event%20Reference%20Structure%20%28by%20ref%29))
  (Utilities|FlowControl|Sequence
    (:then_0
      (Utilities|IsValid MeshComp
        (:Is%20Valid
          (Utilities|IsValid (Components|SkeletalMesh|GetAnimInstance MeshComp)
            (:Is%20Valid
              (Utilities|IsValid (Variables|Default|GetSound)
                (:Is%20Valid
                  (Audio|SpawnSoundAttached (Variables|Default|GetSound) MeshComp (Variables|Default|GetAttach%20Point%20Name) "0, 0, 0" "0, 0, 0" "KeepRelativeOffset" true (Variables|Default|GetVolume%20Multiplier) (Variables|Default|GetPitch%20Multiplier) 0.0 0 0))))))))
    (:then_1
      (return true))))